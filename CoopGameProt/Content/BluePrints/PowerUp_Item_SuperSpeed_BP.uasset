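; Super speed power-up item that temporarily doubles the movement speed of the actor it is activated for.
; On activation it stores that actor and sets its CharacterMovementComponent MaxWalkSpeed to twice the current GetMaxSpeed.
; On expiry it halves the then-current max speed if the actor is still valid, rather than restoring a saved value, then calls the parent's expiry logic.
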(event Collision|EventActorBeginOverlap
  (params (OtherActor :type Actor%20Object%20Reference)))

(event EventOnExpired
  (bind _activatedforplaer (Variables|Default|GetActivatedForPlaer))
  (bind _returnvalue (Actor|GetComponentbyClass _activatedforplaer "/Script/Engine.CharacterMovementComponent"))
  (Utilities|IsValid _activatedforplaer
    (:Is%20Valid
      (Variables|/Script/Engine.CharacterMovementComponent|SetMaxWalkSpeed _returnvalue (/ (Class|MovementComponent|GetMaxSpeed _returnvalue) 2.0)))
    (:Is%20Not%20Valid
      _))
  (|CallParentFunction))

(event EventOnActivated
  (params (ActiveFor :type Actor%20Object%20Reference))
  (bind _returnvalue (Actor|GetComponentbyClass ActiveFor "/Script/Engine.CharacterMovementComponent"))
  (Variables|Default|SetActivatedForPlaer ActiveFor)
  (Variables|/Script/Engine.CharacterMovementComponent|SetMaxWalkSpeed _returnvalue (* (Class|MovementComponent|GetMaxSpeed _returnvalue) 2.0)))

(fn ConstructionScript)